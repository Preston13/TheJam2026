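; BP_RandomizeComponent is a component that randomizes the appearance of the Talker that owns it.
; On BeginPlay it assigns a random skeletal mesh from MeshOptions to the owner's mesh, and does nothing if the owner is not a Talker.
; It then walks the new mesh's material slot names, giving Hair and Shirt slots random materials from their option arrays.
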(event `self.ReceiveBeginPlay`
  (bind _astalker (cast `/Game/Gameplay/Dialogue/Actors/Talker` (`self.GetOwner`)))
  (bind _output_get (set `self.Mesh` (`Character.Mesh` _astalker)))
  (set `SkeletalMeshComponent.SkeletalMeshAsset` (`|GetArrayItem` (`self.MeshOptions`) (`KismetMathLibrary.RandomInteger` (`KismetArrayLibrary.Array_Length` (`self.MeshOptions`)))) _output_get)
  (for (_array_element _array_index) (`PrimitiveComponent.GetMaterialSlotNames` _output_get)
    (switch `name` _array_element
      (:`Hair`
        (`PrimitiveComponent.SetMaterial` (`self.Mesh`) _array_index (`|GetArrayItem` (`self.HairOptions`) (`KismetMathLibrary.RandomInteger` (`KismetArrayLibrary.Array_Length` (`self.HairOptions`))))))
      (:`Shirt`
        (`PrimitiveComponent.SetMaterial` (`self.Mesh`) _array_index (`|GetArrayItem` (`self.ShirtOptions`) (`KismetMathLibrary.RandomInteger` (`KismetArrayLibrary.Array_Length` (`self.ShirtOptions`)))))))))
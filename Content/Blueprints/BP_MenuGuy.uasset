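; Decorative menu character that picks a random skeletal mesh from MeshOptions when play begins.
; It starts by playing a sit-down animation, then alternates between stand-up and sit-down animations indefinitely.
; StandUp and SitDown schedule each other through timers with random delays, so the timing varies.
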(event `self.ReceiveBeginPlay`
  (bind _mesh (`self.Mesh`))
  (set `SkeletalMeshComponent.SkeletalMeshAsset` (`|GetArrayItem` (`self.MeshOptions`) (`KismetMathLibrary.RandomInteger` (`KismetArrayLibrary.Array_Length` (`self.MeshOptions`)))) _mesh)
  (`SkeletalMeshComponent.PlayAnimation` _mesh "/Game/Models/People/BaseCharacter_Anim_CharacterArmature_SitDown.BaseCharacter_Anim_CharacterArmature_SitDown" false)
  (`KismetSystemLibrary.K2_SetTimerDelegate` (delegate `StandUp`) (`KismetMathLibrary.RandomFloatInRange` 1.0 3.0)))

(event `StandUp`
  (`SkeletalMeshComponent.PlayAnimation` (`self.Mesh`) "/Game/Models/People/BaseCharacter_Anim_CharacterArmature_StandUp.BaseCharacter_Anim_CharacterArmature_StandUp" false)
  (`KismetSystemLibrary.K2_SetTimerDelegate` (delegate `SitDown`) (`KismetMathLibrary.RandomFloatInRange` 1.0 5.0)))

(event `SitDown`
  (`SkeletalMeshComponent.PlayAnimation` (`self.Mesh`) "/Game/Models/People/BaseCharacter_Anim_CharacterArmature_SitDown.BaseCharacter_Anim_CharacterArmature_SitDown" false)
  (`KismetSystemLibrary.K2_SetTimerDelegate` (delegate `StandUp`) (`KismetMathLibrary.RandomFloatInRange` 1.0 5.0)))

(fn `UserConstructionScript`)